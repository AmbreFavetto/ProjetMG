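; Player controller for a chess game that turns left mouse clicks into moves on the board.
; On BeginPlay it shows the cursor and caches the first Chess actor in the level.
; On mouse release it bounds-checks the cursor trace hit, forwarding board hits to the Chess actor's Click.
; Off-board hits snap the last clicked piece back to its square, computed from its 8x8 index, and clear the selection.
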(event EventBeginPlay
  (Variables|Default|SetbShowMouseCursor true)
  (bind _outactors (Actor|GetAllActorsOfClass "/Game/Blueprints/Chess.Chess_C"))
  (bind _aschess (Utilities|Casting|CastToChess (Utilities|Array|Get(acopy) _outactors)))
  (Variables|Default|SetchessBoard _aschess))

(event Input|MouseEvents|LeftMouseButton
  (params (Key :type Key%20Structure :default "None"))
  (bind _hitresult (Game|Player|GetHitResultUnderCursorbyChannel "TraceTypeQuery1" true))
  (bind _location (Collision|BreakHitResult _hitresult))
  (:Released
    (Utilities|CheckifYouClickontheBoard _location _location
      (:else
        (Default|Click (Variables|Default|GetchessBoard) _location)))))

(fn ConstructionScript)