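; Menu player controller for the LoupGarou game, handling the lobby, in-game menu and roles HUDs.
; Events reuse or create a widget and add it to the viewport, but only the lobby has a widget class set.
; ShowMenu toggles pause along with the menu, mouse cursor and input mode.
; The menu and roles widget references are set to None, and DisplayErrorMessage is an empty stub.
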(event Custom|HUD%20-%20Roles
  ;[0.3386 1 0.2767] Menu in game
  (Utilities|IsValid (.HUD_Roles (Variables|Default|GetHUD_Roles))
    (:Is%20Valid
      _)
    (:Is%20Not%20Valid
      (bind _returnvalue (UserInterface|CreateWidget 0 (Game|GetPlayerController 0)))
      (bind _output_get (Variables|Default|SetHUD_Roles 0 _returnvalue))))
  (UserInterface|Viewport|AddtoViewport _output_get 0))

(event Custom|HUD%20-%20Menu
  ;[0.3386 1 0.2767] Menu in game
  (Utilities|IsValid (.HUD_Menu (Variables|Default|GetHUD_Menu))
    (:Is%20Valid
      _)
    (:Is%20Not%20Valid
      (bind _returnvalue (UserInterface|CreateWidget 0 (Game|GetPlayerController 0)))
      (bind _output_get (Variables|Default|SetHUD_Menu 0 _returnvalue))))
  (UserInterface|Viewport|AddtoViewport _output_get 0))

(event Custom|HUD%20-%20Lobby
  ;[1 1 1] Connexion
  (Utilities|IsValid (Variables|Default|GetHUD_Lobby)
    (:Is%20Valid
      _)
    (:Is%20Not%20Valid
      (bind _returnvalue (UserInterface|CreateWidget "/Game/HUDS/Lobby/HUD_lobby.HUD_lobby_C" (Game|GetPlayerController 0)))
      (bind _output_get (Variables|Default|SetHUD_Lobby _returnvalue))))
  (UserInterface|Viewport|AddtoViewport _output_get 0))

(fn ConstructionScript)

(fn ShowMenu
  (bind _returnvalue (Game|GetPlayerController 0))
  (bind _returnvalue_2 (Game|GetPlayerController 0))
  (if (Game|IsGamePaused)
    (Game|SetGamePaused false)
    (Widget|RemovefromParent (.HUD_Menu (Variables|Default|GetHUD_Menu)))
    (Variables|/Script/Engine.PlayerController|SetbShowMouseCursor _returnvalue false)
    (Input|SetInputModeGameOnly _returnvalue)
    (else
      (Game|SetGamePaused true)
      (CallFunction|HUD-Menu)
      (Variables|/Script/Engine.PlayerController|SetbShowMouseCursor _returnvalue_2 true)
      (Input|SetInputModeGameandUI _returnvalue_2 0 "LockAlways" false))))