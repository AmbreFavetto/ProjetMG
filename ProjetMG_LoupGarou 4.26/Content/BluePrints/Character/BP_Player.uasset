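; BP_Player is the player Blueprint, handling mouse yaw and a vote against another player.
; Vote requires IsDead on the voter, then ServerVote line-traces from the camera for another BP_Player with IsDead set.
; ServerTouch adds one vote per voter via the Voted flag, and ClientTouch refreshes the target's TxtVotes.
; OpenMenu, ClientDead and DisplayErrorMessage are unfinished stubs.
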(event Custom|ServerVote
  (bind _camera (Variables|Default|GetCamera))
  (bind _returnvalue (Transformation|GetWorldLocation _camera))
  ;[1 0.4351 0.4849] Vote
  (bind _outhit (Collision|LineTraceByChannel _returnvalue (+ _returnvalue (* (Math|Vector|GetForwardVector _camera) 5e+03)) "TraceTypeQuery1" false 0 "None"))
  (bind _asbp_player (Utilities|Casting|CastToBP_Player (.HitActor (Collision|BreakHitResult _outhit))))
  (if (Variables|BP_Player_C|GetisDead _asbp_player)
    (CallFunction|ServerTouch _asbp_player)))

(event Custom|ClientTouch
  (params (VotedPlayer :type BP%20Player%20Object%20Reference))
  ;[1 0.3527 0.3945] Refresh the number of votes
  (Rendering|Components|TextRender|SetText (Variables|BP_Player_C|GettxtVotes VotedPlayer) (Utilities|Text|ToText(Integer) (Variables|BP_Player_C|GetVotes VotedPlayer))))

(event Custom|ServerTouch
  (params (VotedPlayer :type BP%20Player%20Object%20Reference))
  ;[1 0.3527 0.3945] Refresh the number of votes
  (if (Variables|BP_Player_C|GetVoted self)
    (Development|PrintString "déjà voté!")
    (else
      (Variables|BP_Player_C|SetVotes VotedPlayer (+ (Variables|BP_Player_C|GetVotes VotedPlayer) 1))
      (Variables|Default|SetVoted true)))
  (CallFunction|ClientTouch VotedPlayer))

(event Custom|ClientDead
  (params (VotedPlayer :type BP%20Player%20Object%20Reference))
  ;[1 0.3527 0.3945] Refresh the number of votes
  (Utilities|FlowControl|Delay 1e+01))

(event Input|ActionEvents|InputActionOpenMenu
  (params (Key :type Key%20Structure :default "None"))
  ;[1 1 1] Open/Close menu
  (:Pressed
    (Utilities|Casting|CastToBP_GameInfoInstance (Game|GetGameInstance))))

(event Input|ActionEvents|InputActionVote
  (params (Key :type Key%20Structure :default "None"))
  ;[1 0.4351 0.4849] Vote
  (:Pressed
    (if (Variables|Default|GetisDead)
      (CallFunction|ServerVote))))

(event Input|AxisEvents|InputAxisLookSide
  (params (AxisValue :type Float%20%28single-precision%29))
  ;[1 1 1] Mouse Movements
  (Pawn|Input|AddControllerYawInput AxisValue))

(fn ConstructionScript)